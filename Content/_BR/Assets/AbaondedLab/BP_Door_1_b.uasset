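; Automatic double sliding door actor in the AbaondedLab assets that opens and closes around a trigger volume.
; Begin and end overlap each play their own timeline, with no filter on the overlapping actor.
; Each timeline update nudges the two panels oppositely along world X by a fixed offset, so travel depends on frame rate.
; Both timelines use Play without restarting or reversing.
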(event OnComponentBeginOverlap(TriggerVolume)
  (params (OverlappedComponent :type Primitive%20Component%20Object%20Reference) (OtherActor :type Actor%20Object%20Reference) (OtherComp :type Primitive%20Component%20Object%20Reference) (OtherBodyIndex :type Integer) (bFromSweep :type Boolean) (SweepResult :type Hit%20Result%20Structure%20%28by%20ref%29))
  (Timeline|Open Play
    (:Update
      (Transformation|AddWorldOffset (Variables|Default|GetnachYMinus) (Math|Vector|MakeVector -1.7 0.0 0.0) false false)
      (Transformation|AddWorldOffset (Variables|Default|GetnachYPlus) (Math|Vector|MakeVector 1.7 0.0 0.0) false false))))

(event OnComponentEndOverlap(TriggerVolume)
  (params (OverlappedComponent :type Primitive%20Component%20Object%20Reference) (OtherActor :type Actor%20Object%20Reference) (OtherComp :type Primitive%20Component%20Object%20Reference) (OtherBodyIndex :type Integer))
  (Timeline|Timeline_0 Play
    (:Update
      (Transformation|AddWorldOffset (Variables|Default|GetnachYMinus) (Math|Vector|MakeVector 1.7 0.0 0.0) false false)
      (Transformation|AddWorldOffset (Variables|Default|GetnachYPlus) (Math|Vector|MakeVector -1.7 0.0 0.0) false false))))

(event EventBeginPlay)

(event Collision|EventActorBeginOverlap
  (params (OtherActor :type Actor%20Object%20Reference)))

(event EventTick
  (params (DeltaSeconds :type Float%20%28single-precision%29)))

(fn ConstructionScript)