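; Player controller for in-game play that manages weapon preview capture and switches input between UI and gameplay.
; On begin play, the local controller spawns a weapon capture actor high above the level and stores it as WeaponInfo.
; Helper functions add a widget to the viewport with Game and UI input and a visible cursor, or restore game-only input with the cursor hidden.
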(event EventBeginPlay
  ;[1 1 1] Create
  (if (Pawn|IsLocalController)
    (bind _returnvalue (Game|SpawnActorfromClass "/Game/Blueprints/Ingame/BP_WeaponCaptureBlueprint.BP_WeaponCaptureBlueprint_C" (Math|Transform|MakeTransform "0, 0,50000.000000" "90.000000,0.000000, 0" "1,1,1") "Undefined" 0 0))
    (Variables|Default|SetWeaponInfo _returnvalue)))

(fn ConstructionScript)

(fn SetupWidgetFocus
  (params (Widget :type User%20Widget%20Object%20Reference))
  (UserInterface|Viewport|AddtoViewport Widget 0)
  (Variables|Default|SetbShowMouseCursor true)
  (Input|SetInputModeGameandUI self Widget "DoNotLock" false))

(fn SetupGameFocus
  (Variables|Default|SetbShowMouseCursor false)
  (Input|SetInputModeGameOnly self))