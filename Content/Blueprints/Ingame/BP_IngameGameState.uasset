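; BP_IngameGameState is a game state that tracks the match phase through WaitingForPlayers, Starting and Ingame.
; The authority sets WaitingForPlayers on BeginPlay, and an OnGameStarting event switches the phase to Starting.
; During Starting, the authority's Tick counts StartingTimeLeft down and fires OnGameIngame at zero.
; A helper function returns the player count from the PlayerArray length.
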(event Custom|OnGameStarting
  ;[1 1 1] On Starting
  (Variables|Default|SetCurrentGameState "NewEnumerator2"))

(event Custom|OnGameIngame
  ;[1 1 1] Ingame
  (Variables|Default|SetCurrentGameState "NewEnumerator3"))

(event EventBeginPlay
  ;[1 1 1] Begin play
  (Networking|SwitchHasAuthority
    (:Authority
      (Variables|Default|SetCurrentGameState "NewEnumerator1"))))

(event EventTick
  (params (DeltaSeconds :type Float%20%28single-precision%29))
  ;[1 1 1] Tick
  (Networking|SwitchHasAuthority
    (:Authority
      (switch Utilities|FlowControl|Switch|SwitchonE_GameState (Variables|Default|GetCurrentGameState)
        (:NewEnumerator2
          ;[1 1 1] Starting
          (bind _output_get (Variables|Default|SetStartingTimeLeft (- (Variables|Default|GetStartingTimeLeft) DeltaSeconds)))
          (if (<= _output_get 0.0)
            (CallFunction|OnGameIngame)))))))

(fn ConstructionScript)

(fn GetPlayerCount
  (return (Utilities|Array|Length (Variables|Default|GetPlayerArray))))