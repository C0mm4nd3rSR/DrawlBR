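; BP_AmmoPickUp is an ammo pickup that gives ammo to a player character on touch.
; Tick spins its static mesh around yaw at RotationSpeed.
; Box overlap runs only on authority, casts the other actor to BP_IngameCharacter, calls OCAddAmmo with the configured ammo type and amount, then destroys the pickup.
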(event OnComponentBeginOverlap(Box)
  (params (OverlappedComponent :type Primitive%20Component%20Object%20Reference) (OtherActor :type Actor%20Object%20Reference) (OtherComp :type Primitive%20Component%20Object%20Reference) (OtherBodyIndex :type Integer) (bFromSweep :type Boolean) (SweepResult :type Hit%20Result%20Structure%20%28by%20ref%29))
  ;[1 1 1] Add Ammo
  (Networking|SwitchHasAuthority
    (:Authority
      (bind _asbp_ingame_character (Utilities|Casting|CastToBP_IngameCharacter OtherActor))
      (Default|OCAddAmmo _asbp_ingame_character (Variables|Default|GetE_AmmoType) (Variables|Default|GetAmmoAmount))
      (Actor|DestroyActor))))

(event EventTick
  (params (DeltaSeconds :type Float%20%28single-precision%29))
  ;[1 1 1] Rotate
  (Transformation|AddRelativeRotation (Variables|Default|GetStaticMesh) (Math|Rotator|MakeRotator 0.0 0.0 (* DeltaSeconds (Variables|Default|GetRotationSpeed))) false false))

(fn ConstructionScript)