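; BP_Bullet is an in-game bullet actor that detects impacts along its flight path and destroys itself on hit.
; BeginPlay starts a looping timer that calls Update, which line-traces from the last recorded position to the current one, covering the gap between ticks.
; A hit on world, pawn or physics objects draws a red debug point and destroys the actor; the graphs apply no damage or movement.
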(event EventBeginPlay
  ;[1 1 1] Init
  (Utilities|Time|SetTimerbyFunctionName self "Update" 0.05 true)
  (Variables|Default|SetLastPos (Transformation|GetActorLocation)))

(fn ConstructionScript)

(fn Update
  ;[1 1 1] Update
  (Utilities|FlowControl|Sequence
    (:then_0
      ;[1 1 1] Bullet
      (bind (_outhit _returnvalue) (Collision|LineTraceForObjects (Variables|Default|GetLastPos) (Transformation|GetActorLocation) (Utilities|Array|MakeArray "ObjectTypeQuery1" "ObjectTypeQuery2" "ObjectTypeQuery3" "ObjectTypeQuery4") false 0 "None" true "(R=1.000000,G=0.000000,B=0.000000,A=1.000000)" "(R=0.000000,G=1.000000,B=0.000000,A=1.000000)" 1e+02))
      (if _returnvalue
        (Rendering|Debug|DrawDebugPoint (.Location (Collision|BreakHitResult _outhit)) 1e+01 "(R=1.000000,G=0.015625,B=0.015625,A=1.000000)" 1e+01)
        (Actor|DestroyActor)))
    (:then_1
      ;[1 1 1] Update Last Pos
      (Variables|Default|SetLastPos (Transformation|GetActorLocation)))))